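; Small bomb enemy that is knocked back when damaged and explodes after a lit fuse.
; Any damage launches it away via KnockBack and sparks it, with a DoOnce starting a single, slightly randomized fuse timer that calls ExplodeSelf.
; While sparked, hitting an actor that implements BPI_Enemies sends that actor KnockBackNoFuseMessage, passing itself.
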(event `self.ReceiveAnyDamage`
  (params (Damage :type "Float (single-precision)") (DamageType :type "DamageType Object Reference") (InstigatedBy :type "Controller Object Reference") (DamageCauser :type "Actor Object Reference"))
  ; When Bomb Enemy is hit, It will be Launched in the direction the player hit it
  (`self.KnockBack` DamageCauser)
  (set `self.IsSparked?` true)
  (`/Engine/EditorBlueprintResources/StandardMacros.DoOnce` false
    (:`Completed`
      (`KismetSystemLibrary.K2_SetTimerDelegate` (delegate `FuseLit`) (+ (`self.FuseDuration`) (`KismetMathLibrary.RandomFloatInRange` -0.5 0.5))))))

(event `FuseLit`
  ; When Bomb Enemy is hit, It will be Launched in the direction the player hit it
  (`self.ExplodeSelf`))

(event `self.ReceiveHit`
  (params (MyComp :type "PrimitiveComponent Object Reference") (Other :type "Actor Object Reference") (OtherComp :type "PrimitiveComponent Object Reference") (bSelfMoved :type Boolean) (HitLocation :type "Vector Structure") (HitNormal :type "Vector Structure") (NormalImpulse :type "Vector Structure") (Hit :type "HitResult Structure (by ref)"))
  (if (and (`KismetSystemLibrary.DoesImplementInterface` Other "/Game/Enemies/BPI_Enemies.BPI_Enemies_C") (`self.IsSparked?`))
    (message `/Game/Enemies/BPI_Enemies.KnockBackNoFuse` Other self)))

(fn `UserConstructionScript`
  (`parent.UserConstructionScript`))
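; Bottle rocket projectile that flies with optional homing and explodes on impact or after a fixed fuse timer.
; BeginPlay either assigns the homing target component or zeroes homing acceleration, then starts the timer.
; The explosion sphere-traces for pawns, skipping itself, its instigator and player 0, damages each actor once, then destroys the rocket.
; An Exploded flag guards repeat hits, and the trace leaves persistent debug drawing enabled.
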(event `self.ReceiveBeginPlay`
  (`|ExecutionSequence`
    (:`then_0`
      (if (`self.IsHoming?`)
        (set `ProjectileMovementComponent.HomingTargetComponent` (`self.HomingTargetEnemyComponent`) (`self.ProjectileMovement`))
        (else
          (set `ProjectileMovementComponent.HomingAccelerationMagnitude` 0.0 (`self.ProjectileMovement`)))))
    (:`then_1`
      (`KismetSystemLibrary.K2_SetTimerDelegate` (delegate `Explode`) 5.0))))

(event `Explode`
  (bind _returnvalue (`self.K2_GetActorLocation`))
  (bind _hitenemiesarray (`self.HitEnemiesArray`))
  (set `self.Exploded?` true :!label _label)
  (bind _outhits (`KismetSystemLibrary.SphereTraceMultiForObjects` _returnvalue _returnvalue 300.0 (`|MakeArray` "ObjectTypeQuery3" :!type "EObjectTypeQuery Enum") false (`|MakeArray` self (`self.Instigator`) (`GameplayStatics.GetPlayerCharacter` 0) :!type "Actor Object Reference") "Persistent"))
  (for _array_element _outhits
    (bind (_bblockinghit _binitialoverlap _time _distance _location _impactpoint _normal _impactnormal _physmat _hitactor) (`GameplayStatics.BreakHitResult` _array_element))
    (if (not (`KismetArrayLibrary.Array_Contains` _hitenemiesarray _hitactor))
      (`KismetArrayLibrary.Array_Add` _hitenemiesarray _hitactor)
      (`GameplayStatics.ApplyDamage` _hitactor 10.0 null self)))
  (`KismetArrayLibrary.Array_Clear` _hitenemiesarray)
  (`self.K2_DestroyActor`))

(event `self.ReceiveHit`
  (params (MyComp :type "PrimitiveComponent Object Reference") (Other :type "Actor Object Reference") (OtherComp :type "PrimitiveComponent Object Reference") (bSelfMoved :type Boolean) (HitLocation :type "Vector Structure") (HitNormal :type "Vector Structure") (NormalImpulse :type "Vector Structure") (Hit :type "HitResult Structure (by ref)"))
  (if (not (`self.Exploded?`))
    (goto _label)))

(fn `UserConstructionScript`)
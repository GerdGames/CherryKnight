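; BP_EnemyBaseClass is the base enemy Blueprint, tying each enemy into wave tracking, AI and the Gameplay Ability System.
; BeginPlay registers it with the WaveManagerSubsystem, runs its behavior tree and binds the health bar widget to its AbilitySystemComponent.
; Destroyed unregisters it from the wave manager.
; ExplodeSelf and KnockBack are empty, with their radial damage and launch logic left disconnected.
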(event `self.ReceiveBeginPlay`
  (`parent.ReceiveBeginPlay`)
  (`WaveManager_Subsystem.AddActiveEnemy` (subsystem `WaveManager_Subsystem`) self)
  (`AIController.RunBehaviorTree` (`AIBlueprintHelperLibrary.GetAIController` self) (`self.Behavior Tree`))
  (`self.InitHealthBar`))

(event `self.ReceiveDestroyed`
  (`WaveManager_Subsystem.RemoveActiveEnemy` (subsystem `WaveManager_Subsystem`) self))

(fn `ExplodeSelf`)

(fn `InitHealthBar`
  (bind _aswbp_gas_base (cast `/Game/UI/WBP_GasBase` (`WidgetComponent.GetWidget` (`self.Widget`))))
  (`GSCUserWidget.InitializeWithAbilitySystem` _aswbp_gas_base (`self.AbilitySystemComponent`)))

(fn `KnockBack`
  (params (DamageCauser :type "Actor Object Reference")))

(fn `UserConstructionScript`)
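; Base gameplay ability providing shared combat helpers, with no activation logic of its own.
; DealDamage applies normal or blast damage via SetByCaller effects, then optionally lights a fuse on non-immune, non-player targets and sends a knockback event.
; If health dropped, optional hit stop hits the ability's avatar and a hit-react event goes to the target.
; RedFlash toggles custom depth stencil on character or pillar meshes; ExtinguishFuse is disconnected.
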(fn `DealDamage`
  (params (Actor :type "Actor Object Reference") (Damage :type "Float (double-precision)") (`LightFuse?` :type Boolean) (`IsBlastDamage?` :type Boolean) (`KnockBack?` :type Boolean) (KnockMagnitude :type "Float (double-precision)") (HitStopDuration :type "Float (double-precision)" :default 0.01) (`AppliesHitStop?` :type Boolean))
  (locals (Lcl_StoredHP :type "Float (single-precision)"))
  (bind _returnvalue (`AbilitySystemBlueprintLibrary.GetAbilitySystemComponent` Actor))
  (`/Engine/EditorBlueprintResources/StandardMacros.IsValid` _returnvalue
    (:`Is Valid`
      (set `local.Lcl_StoredHP` (`.ReturnValue` (`AbilitySystemComponent.GetGameplayAttributeValue` _returnvalue (struct :`AttributeName` "CurrentHealth" :`Attribute` "/Game/GAS/Attributes/GBA_AttributesBase.GBA_AttributesBase_C:CurrentHealth" :`AttributeOwner` "/Script/Engine.BlueprintGeneratedClass'/Game/GAS/Attributes/GBA_AttributesBase.GBA_AttributesBase_C'"))))
      (bind _result (`/Engine/EditorBlueprintResources/StandardMacros.NegateFloat` Damage)
        (:`  `
          (`|ExecutionSequence`
            (:`then_0`
              (bind _returnvalue_2 (`AbilitySystemBlueprintLibrary.AssignTagSetByCallerMagnitude` (`self.MakeOutgoingGameplayEffectSpec` (select `bool` `IsBlastDamage?` :`false` "/Game/GAS/Effects/GE_Damage.GE_Damage_C" :`true` "/Game/GAS/Effects/GE_BlastDamage.GE_BlastDamage_C" :!type "GameplayEffect Class Reference")) (struct :`TagName` "Attack.Damage") _result))
              (`self.K2_ApplyGameplayEffectSpecToTarget` _returnvalue_2 (`AbilitySystemBlueprintLibrary.AbilityTargetDataFromActor` Actor))
              (`GameplayStatics.ApplyDamage` Actor 1.0 null (`self.GetAvatarActorFromActorInfo`)))
            (:`then_1`
              (if `LightFuse?`
                (`self.LightFuse` Actor)
                (else
                  (`self.ExtinguishFuse` Actor))))
            (:`then_2`
              (if `KnockBack?`
                (`self.KnockBack` Actor KnockMagnitude)))
            (:`then_3`
              (if `AppliesHitStop?`
                (if (< (`.ReturnValue` (`AbilitySystemComponent.GetGameplayAttributeValue` (`AbilitySystemBlueprintLibrary.GetAbilitySystemComponent` Actor) (struct :`AttributeName` "CurrentHealth" :`Attribute` "/Game/GAS/Attributes/GBA_AttributesBase.GBA_AttributesBase_C:CurrentHealth" :`AttributeOwner` "/Script/Engine.BlueprintGeneratedClass'/Game/GAS/Attributes/GBA_AttributesBase.GBA_AttributesBase_C'"))) (`local.Lcl_StoredHP`))
                  (bind _returnvalue_3 (`AbilitySystemBlueprintLibrary.AssignTagSetByCallerMagnitude` (`self.MakeOutgoingGameplayEffectSpec` "/Game/GAS/Effects/Player/GE_HitStop.GE_HitStop_C") (struct :`TagName` "Event.HitStop.Duration") HitStopDuration))
                  (`self.K2_ApplyGameplayEffectSpecToTarget` _returnvalue_3 (`AbilitySystemBlueprintLibrary.AbilityTargetDataFromActor` (`.AvatarActor` (break `GameplayAbilityActorInfo` (`self.GetActorInfo`)))))
                  (`AbilitySystemBlueprintLibrary.SendGameplayEventToActor` Actor (struct :`TagName` "Character.Hit.React") (make `GameplayEventData` (struct))))))))))))

(fn `ExtinguishFuse`
  (params (Actor :type "Actor Object Reference")))

(fn `KnockBack`
  (params (Actor :type "Actor Object Reference") (KnockMagnitude :type "Float (single-precision)" :default 500.0))
  (`AbilitySystemBlueprintLibrary.SendGameplayEventToActor` Actor (struct :`TagName` "Character.Hit.Knockback") (make `GameplayEventData` (struct :`TagName` "Character.Hit.Knockback") (`self.GetAvatarActorFromActorInfo`) Actor null null (struct) (struct) (struct) KnockMagnitude)))

(fn `LightFuse`
  (params (Actor :type "Actor Object Reference"))
  (bind _returnvalue (`AbilitySystemBlueprintLibrary.GetAbilitySystemComponent` Actor))
  (`/Engine/EditorBlueprintResources/StandardMacros.IsValid` Actor
    (:`Is Valid`
      (`/Engine/EditorBlueprintResources/StandardMacros.IsValid` _returnvalue
        (:`Is Valid`
          (if (and (!= Actor (`GameplayStatics.GetPlayerCharacter` 0)) (not (`GameplayTagAssetInterface.HasAnyMatchingGameplayTags` _returnvalue (`BlueprintGameplayTagLibrary.MakeLiteralGameplayTagContainer` (struct :`GameplayTags` (struct :`(TagName` "Character.Enemy.Fuse.Immune") :`(TagName` "Character.Enemy.Fuse.Lit")))))))
            (`self.K2_ApplyGameplayEffectSpecToTarget` (`self.MakeOutgoingGameplayEffectSpec` "/Game/GAS/Effects/Enemy/GE_FuseLit.GE_FuseLit_C") (`AbilitySystemBlueprintLibrary.AbilityTargetDataFromActor` Actor))
            (`AbilitySystemBlueprintLibrary.AddLooseGameplayTags` Actor (`BlueprintGameplayTagLibrary.MakeLiteralGameplayTagContainer` (struct :`GameplayTags` (struct :`(TagName` "Character.Enemy.Fuse.Lit")))))))))))

(fn `RedFlash`
  (params (`StartFlash?` :type Boolean))
  (bind _returnvalue (`self.GetAvatarActorFromActorInfo`))
  (bind _ascharacter (cast `Character` _returnvalue)
    (:`then`
      (`PrimitiveComponent.SetCustomDepthStencilValue` (`Character.Mesh` _ascharacter) (`KismetMathLibrary.SelectInt` 1 0 `StartFlash?`)))
    (:`CastFailed`
      (bind _asbp_pillar (cast `/Game/Blueprints/Pillars/BP_Pillar` _returnvalue))
      (`PrimitiveComponent.SetCustomDepthStencilValue` (`/Game/Blueprints/Pillars/BP_Pillar.Pillar_Mesh` _asbp_pillar) (`KismetMathLibrary.SelectInt` 1 0 `StartFlash?`)))))
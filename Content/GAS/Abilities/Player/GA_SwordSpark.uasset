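; Player gameplay ability for a heavy sword attack with a spark effect, built on the KnightHeavyAttack montage.
; Activation plays the montage with layered attack sounds.
; The montage's notify event spawns an oversized damage hitbox with knockback and hitstop attached to the right hand, adds the SwordSparks gameplay cue, plays a boom and locks movement input.
; Ability end restores movement, removes the cue and destroys the hitbox.
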(event `self.K2_ActivateAbility`
  (bind (_skeletal _sword) (`self.GetSockets`))
  (bind _owneractor (break `GameplayAbilityActorInfo` (`self.GetActorInfo`)))
  (bind (_owneractor_2 _avataractor _playercontroller) (break `GameplayAbilityActorInfo` (`self.GetActorInfo`)))
  (bind _returnvalue (`Actor.K2_GetActorLocation` _owneractor))
  (`parent.K2_ActivateAbility`)
  (`GSCTask_PlayMontageWaitForEvent.PlayMontageAndWaitForEvent` "None" "/Game/Art/Mesh/Character/Knight/KnightHeavyAttack.KnightHeavyAttack" (struct :`GameplayTags` (struct :`(TagName` "Event.Anim.Notify")))
    (:`then`
      ; Play Sound
      (bind _asbp_character_base (cast `/Game/Characters/BP_CharacterBase` _owneractor))
      (`GameplayStatics.PlaySoundAtLocation` (`/Game/Characters/BP_CharacterBase.AttackSoundCue` _asbp_character_base) _returnvalue (struct) 1.0 1.0 0.0 null null null null)
      (`KismetSystemLibrary.Delay` 0.2)
      (`GameplayStatics.PlaySoundAtLocation` "/Game/Audio/Player/Sword/HeavySwordCue.HeavySwordCue" _returnvalue (struct) 1.0 1.0 0.0 null null null null))
    (:`OnCompleted`
      (`self.K2_EndAbility` :!label _label))
    (:`OnBlendOut`
      (goto _label))
    (:`OnInterrupted`
      (goto _label))
    (:`EventReceived`
      (bind _returnvalue_2 (`|SpawnActorFromClass` "/Game/Blueprints/Hitboxes/Hitbox.Hitbox_C" (`KismetMathLibrary.MakeTransform` (.location _sword) (.rotation _sword) (8.0 8.0 8.0)) "Undefined" "MultiplyWithRoot" null 10.0 true false self true 600.0 0.02 true null))
      (`Actor.K2_AttachToComponent` _returnvalue_2 _skeletal "RightHand" "KeepWorld" "KeepWorld" "KeepWorld" true)
      (set `self.HitBoxActor` _returnvalue_2)
      (`GSCBlueprintFunctionLibrary.AddGameplayCue` (`self.GetAvatarActorFromActorInfo`) (struct :`TagName` "GameplayCue.Attack.SwordSparks"))
      (`GameplayStatics.PlaySoundAtLocation` "/Game/Audio/Enemies/Explosions/BigBoom.BigBoom" (`Actor.K2_GetActorLocation` _owneractor_2) (struct) 4.0 1.0 0.0 null null null null)
      (`Controller.SetIgnoreMoveInput` _playercontroller true))))

(event `self.K2_OnEndAbility`
  (params (bWasCancelled :type Boolean))
  (bind (_owneractor _avataractor _playercontroller) (break `GameplayAbilityActorInfo` (`self.GetActorInfo`)))
  (`parent.K2_OnEndAbility` bWasCancelled)
  (`|ExecutionSequence`
    (:`then_0`
      ; Resume Movement
      (`/Engine/EditorBlueprintResources/StandardMacros.IsValid` _playercontroller
        (:`Is Valid`
          (`Controller.ResetIgnoreMoveInput` _playercontroller))))
    (:`then_1`
      (`GSCBlueprintFunctionLibrary.RemoveGameplayCue` (`self.GetAvatarActorFromActorInfo`) (struct :`TagName` "GameplayCue.Attack.SwordSparks"))
      (bind _hitboxactor (`self.HitBoxActor`)
        (:`then`
          (`Actor.K2_DestroyActor` _hitboxactor))
        (:`else`)))))
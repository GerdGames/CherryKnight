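; Player gameplay ability for a shield slam: a forward leap that lands in a large hitbox with knockback and hitstop.
; A montage starts alongside a root motion jump force, and landing replays it from its "Slam" section while spawning the hitbox, sparks cue and boom.
; Move input locks on impact until an anim notify event or montage exit.
; Self collision is ignored until ability end, which also clears the cue and hitbox.
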(event `self.K2_ActivateAbilityFromEvent`
  (params (EventData :type "GameplayEventData Structure (by ref)"))
  (bind (_skeletal _sword _lefthand _root) (`self.GetSockets`))
  (bind _owneractor (break `GameplayAbilityActorInfo` (`self.GetActorInfo`)))
  (bind (_owneractor_2 _avataractor _playercontroller) (break `GameplayAbilityActorInfo` (`self.GetActorInfo`)))
  (bind (_owneractor_3 _avataractor_2 _playercontroller_2) (break `GameplayAbilityActorInfo` (`self.GetActorInfo`)))
  (bind _returnvalue (`Actor.K2_GetActorLocation` _owneractor))
  (`parent.K2_ActivateAbilityFromEvent` EventData)
  (`self.SetSelfCollision` "ECR_Ignore")
  (`GSCTask_PlayMontageWaitForEvent.PlayMontageAndWaitForEvent` "None" (`self.Montage to Play`) (struct :`GameplayTags` (struct :`(TagName` "Event.Anim.Notify")))
    (:`then`
      (`AbilityTask_ApplyRootMotionJumpForce.ApplyRootMotionJumpForce` "None" (`KismetMathLibrary.Conv_VectorToRotator` (`Actor.GetActorForwardVector` (`self.GetAvatarActorFromActorInfo`))) 100.0 500.0 0.8 0.0 true "MaintainLastRootMotionVelocity"
        (:`then`
          ; Play Sound
          (bind _asbp_character_base (cast `/Game/Characters/BP_CharacterBase` _owneractor))
          (`GameplayStatics.PlaySoundAtLocation` (`/Game/Characters/BP_CharacterBase.AttackSoundCue` _asbp_character_base) _returnvalue (struct) 1.0 1.0 0.0 null null null null)
          (`KismetSystemLibrary.Delay` 0.2)
          (`GameplayStatics.PlaySoundAtLocation` "/Game/Audio/Player/Sword/HeavySwordCue.HeavySwordCue" _returnvalue (struct) 1.0 1.0 0.0 null null null null))
        (:`OnLanded`
          (`GSCTask_PlayMontageWaitForEvent.PlayMontageAndWaitForEvent` "None" (`self.Montage to Play`) (struct :`GameplayTags` (struct :`(TagName` "Event.Anim.Notify"))) 1.0 "Slam"
            (:`then`
              (bind _returnvalue_2 (`|SpawnActorFromClass` "/Game/Blueprints/Hitboxes/Hitbox.Hitbox_C" (`KismetMathLibrary.MakeTransform` (+ (.location _root) (* (`KismetMathLibrary.GetForwardVector` (.rotation _root)) 50.0)) (struct) (12.0 12.0 12.0)) "Undefined" "MultiplyWithRoot" null 5.0 true false self true 750.0 0.02 true null))
              (bind _output_get (set `self.HitBoxActor` _returnvalue_2))
              (`Actor.SetLifeSpan` _output_get 0.3)
              (`GSCBlueprintFunctionLibrary.AddGameplayCue` (`self.GetAvatarActorFromActorInfo`) (struct :`TagName` "GameplayCue.Attack.ShieldSlamSparks"))
              (`GameplayStatics.PlaySoundAtLocation` "/Game/Audio/Enemies/Explosions/BigBoom.BigBoom" (`Actor.K2_GetActorLocation` _owneractor_2) (struct) 4.0 0.5 0.0 null null null null)
              (`Controller.SetIgnoreMoveInput` _playercontroller true))
            (:`OnCompleted`
              (`Controller.ResetIgnoreMoveInput` _playercontroller_2 :!label _label)
              (`self.K2_EndAbility`))
            (:`OnBlendOut`
              (goto _label))
            (:`OnInterrupted`
              (goto _label))
            (:`EventReceived`
              ; Resume Movement
              (`Controller.ResetIgnoreMoveInput` _playercontroller_2))))))))

(event `self.K2_OnEndAbility`
  (params (bWasCancelled :type Boolean))
  (`parent.K2_OnEndAbility` bWasCancelled)
  (`self.SetSelfCollision` "ECR_Block")
  (`GSCBlueprintFunctionLibrary.RemoveGameplayCue` (`self.GetAvatarActorFromActorInfo`) (struct :`TagName` "GameplayCue.Attack.ShieldSlamSparks"))
  (bind _hitboxactor (`self.HitBoxActor`)
    (:`then`
      (`Actor.K2_DestroyActor` _hitboxactor))
    (:`else`)))
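; GA_Block is a player gameplay ability for a held block.
; On activation it saves and halves the avatar's max walk speed, applies GE_Blocking to the owner and plays the knight block montage.
; Releasing the input ends the ability, which restores the saved speed, removes the effect by handle and plays the montage's End section, set to continue after the ability ends.
; Debug strings print on block start and end.
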(event `self.K2_ActivateAbility`
  (bind _returnvalue (`Actor.GetComponentByClass` (`self.GetAvatarActorFromActorInfo`) "/Script/Engine.CharacterMovementComponent"))
  (`parent.K2_ActivateAbility`)
  (bind _output_get (set `self.SavedSpeed` (`CharacterMovementComponent.MaxWalkSpeed` _returnvalue)))
  (set `CharacterMovementComponent.MaxWalkSpeed` (/ _output_get 2.0) _returnvalue)
  (`AbilityTask_WaitInputRelease.WaitInputRelease` false
    (:`then`
      (bind _returnvalue_2 (`self.BP_ApplyGameplayEffectToOwner` "/Game/GAS/Effects/Player/GE_Blocking.GE_Blocking_C"))
      (`KismetSystemLibrary.PrintString` "YOURE ABSOLUTELY TOTALLY BLOCKING RIGHT NOW")
      (`AbilityTask_PlayMontageAndWait.CreatePlayMontageAndWaitProxy` "None" "/Game/Art/Mesh/Character/Knight/KnightBlock_Montage.KnightBlock_Montage"))
    (:`OnRelease`
      (`self.K2_EndAbility`))))

(event `self.K2_OnEndAbility`
  (params (bWasCancelled :type Boolean))
  (`parent.K2_OnEndAbility` bWasCancelled)
  (set `CharacterMovementComponent.MaxWalkSpeed` (`self.SavedSpeed`) (`Actor.GetComponentByClass` (`self.GetAvatarActorFromActorInfo`) "/Script/Engine.CharacterMovementComponent"))
  (`self.BP_RemoveGameplayEffectFromOwnerWithHandle` (stale `self.K2_ActivateAbility` _returnvalue_2))
  (`KismetSystemLibrary.PrintString` "You aint blocking no more")
  (`AbilityTask_PlayMontageAndWait.CreatePlayMontageAndWaitProxy` "None" "/Game/Art/Mesh/Character/Knight/KnightBlock_Montage.KnightBlock_Montage" 1.0 "End" false))
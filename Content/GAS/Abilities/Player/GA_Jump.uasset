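; Gameplay Ability that makes the Cherry Knight player jump with separate rising and falling gravity, noted as currently unused but kept in case movement tags need separating.
; Activation starts the jump, sets the rising gravity scale and binds to the character's jump-apex event.
; At the apex it unbinds and switches to falling gravity.
; Input release stops jumping and ends the ability, allowing variable jump height.
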(event `self.K2_ActivateAbility`
  ; Not currently in use but could be helpful if we need to separate movement tags
  (`parent.K2_ActivateAbility`)
  (bind _asbp_cherry_knight_player (cast `/Game/Characters/BP_CherryKnightPlayer` (`self.GetAvatarActorFromActorInfo`)))
  (`AbilityTask_WaitInputRelease.WaitInputRelease` false
    (:`then`
      (`Character.Jump` _asbp_cherry_knight_player)
      (add `Character.OnReachedJumpApex` _asbp_cherry_knight_player (delegate `UpdateApexGravity`))
      (set `CharacterMovementComponent.GravityScale` (`self.RisingGravity`) (`Character.CharacterMovement` _asbp_cherry_knight_player)))
    (:`OnRelease`
      (`Character.StopJumping` _asbp_cherry_knight_player)
      (`self.K2_EndAbility`))))

(event `UpdateApexGravity`
  ; Not currently in use but could be helpful if we need to separate movement tags
  (remove `Character.OnReachedJumpApex` (stale `self.K2_ActivateAbility` _asbp_cherry_knight_player) (delegate `UpdateApexGravity`))
  (set `CharacterMovementComponent.GravityScale` (`self.FallingGravity`) (`Character.CharacterMovement` (stale `self.K2_ActivateAbility` _asbp_cherry_knight_player))))

(event `self.K2_OnEndAbility`
  (params (bWasCancelled :type Boolean))
  ; Not currently in use but could be helpful if we need to separate movement tags
  (`parent.K2_OnEndAbility` bWasCancelled))
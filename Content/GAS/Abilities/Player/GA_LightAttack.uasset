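; Player Gameplay Ability for a sword light attack that cycles through a montage combo.
; Activation plays the current combo montage and slash sound; montage notify events spawn a Hitbox carrying that step's damage, attached to the right hand.
; Ending destroys the hitbox, advances or wraps the combo index unless cancelled, and starts a short delay that resets the combo.
; Reactivation ends that pending reset to continue the chain.
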(event `self.K2_ActivateAbility`
  (bind (_skeletal _sword) (`self.GetSockets`))
  (`parent.K2_ActivateAbility`)
  (bind _task_comboreset (`self.Task_ComboReset`)
    (:`then`
      (`GameplayTask.EndTask` _task_comboreset))
    (:`else`
      _))
  (`GSCTask_PlayMontageWaitForEvent.PlayMontageAndWaitForEvent` "None" (`|GetArrayItem` (`self.Montage to Play`) (`self.CurrentCombo`)) (struct :`GameplayTags` (struct :`(TagName` "Event.Anim.Notify"))) 1.0 "None" true 0.0
    (:`then`
      (`GameplayStatics.PlaySoundAtLocation` "/Game/Audio/Player/Sword/SwordSlash_Cue.SwordSlash_Cue" (`Actor.K2_GetActorLocation` (`self.GetOwningActorFromActorInfo`)) (struct) 1.0 1.0 0.0 null null null null))
    (:`OnCompleted`
      (`self.K2_EndAbility` :!label _label))
    (:`OnBlendOut`
      (goto _label))
    (:`OnInterrupted`
      (goto _label))
    (:`OnCancelled`
      (goto _label))
    (:`EventReceived`
      (bind _returnvalue (`|SpawnActorFromClass` "/Game/Blueprints/Hitboxes/Hitbox.Hitbox_C" (`KismetMathLibrary.MakeTransform` (.location _sword) (.rotation _sword) (5.0 5.0 5.0)) "Undefined" "MultiplyWithRoot" null (`|GetArrayItem` (`self.DamagePerCombo`) (`self.CurrentCombo`)) false false self true 500.0 0.007 false null))
      (`Actor.K2_AttachToComponent` _returnvalue _skeletal "RightHand" "KeepWorld" "KeepWorld" "KeepWorld" true)
      (set `self.HitBoxActor` _returnvalue))))

(event `self.K2_OnEndAbility`
  (params (bWasCancelled :type Boolean))
  (bind _returnvalue (+ (`self.CurrentCombo`) 1))
  (`parent.K2_OnEndAbility` bWasCancelled)
  (`|ExecutionSequence`
    (:`then_0`
      (bind _hitboxactor (`self.HitBoxActor`)
        (:`then`
          (`Actor.K2_DestroyActor` _hitboxactor))
        (:`else`
          _))
      (bind _asynctaskproxy (`GameplayTask_WaitDelay.TaskWaitDelay` null 1.0)
        (:`then`
          (set `self.Task_ComboReset` _asynctaskproxy))
        (:`OnFinish`
          (set `self.CurrentCombo` 0))))
    (:`then_1`
      (if (not bWasCancelled)
        (set `self.CurrentCombo` (`KismetMathLibrary.SelectInt` _returnvalue 0 (`KismetArrayLibrary.Array_IsValidIndex` (`self.Montage to Play`) _returnvalue)))))))
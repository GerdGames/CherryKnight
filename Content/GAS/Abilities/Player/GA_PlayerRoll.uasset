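; Gameplay Ability for the Cherry Knight player's roll: a dash that knocks back without dealing damage.
; It ignores self collision, plays a shield bash montage unless already attacking, then applies constant-force root motion along move input, or camera forward when stationary.
; An active shield slam makes the force additive and longer.
; An attached hitbox carries the knockback; ending the ability destroys it and restores collision and move input.
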(event `self.K2_ActivateAbility`
  (bind _returnvalue (`self.GetAvatarActorFromActorInfo`))
  (bind _returnvalue_2 (`self.GetAvatarActorFromActorInfo`))
  (`parent.K2_ActivateAbility`)
  (bind _asbp_cherry_knight_player (cast `/Game/Characters/BP_CherryKnightPlayer` (`self.GetAvatarActorFromActorInfo`)))
  (`self.SetSelfCollision` "ECR_Ignore")
  (if (not (`GSCBlueprintFunctionLibrary.HasAnyMatchingGameplayTag` _returnvalue (struct :`GameplayTags` (struct :`(TagName` "Attack") :`(TagName` "Character.Player.Blocking")))))
    (`AbilityTask_PlayMontageAndWait.CreatePlayMontageAndWaitProxy` "None" "/Game/Art/Mesh/Character/Knight/KnightShieldBash.KnightShieldBash"
      (:`then`
        _)))
  (if (`GSCBlueprintFunctionLibrary.HasMatchingGameplayTag` _returnvalue (struct :`TagName` "Attack.Shield.Slam"))
    (set `self.RootMotionIsAdditive?` true)
    (set `self.RootMotionDuration` 0.35)
    (`KismetSystemLibrary.PrintString` "has shield slam tag")
    (else
      (set `self.RootMotionIsAdditive?` false)
      (set `self.RootMotionDuration` 0.25)))
  (`AbilityTask_ApplyRootMotionConstantForce.ApplyRootMotionConstantForce` "None" (`KismetMathLibrary.MakeVector` (.x (`KismetMathLibrary.SelectVector` (`KismetMathLibrary.Normal` (`/Game/Characters/BP_CherryKnightPlayer.MoveInputVector` _asbp_cherry_knight_player)) (`Actor.GetActorForwardVector` (`GameplayStatics.GetPlayerCameraManager` 0)) (!= (`KismetMathLibrary.MakeVector` (.x (`Actor.GetVelocity` _asbp_cherry_knight_player)) (.y (`Actor.GetVelocity` _asbp_cherry_knight_player))) (0.0 0.0 0.0) :`ErrorTolerance` 0.01))) (.y (`KismetMathLibrary.SelectVector` (`KismetMathLibrary.Normal` (`/Game/Characters/BP_CherryKnightPlayer.MoveInputVector` _asbp_cherry_knight_player)) (`Actor.GetActorForwardVector` (`GameplayStatics.GetPlayerCameraManager` 0)) (!= (`KismetMathLibrary.MakeVector` (.x (`Actor.GetVelocity` _asbp_cherry_knight_player)) (.y (`Actor.GetVelocity` _asbp_cherry_knight_player))) (0.0 0.0 0.0) :`ErrorTolerance` 0.01)))) 3000.0 (`self.RootMotionDuration`) (`self.RootMotionIsAdditive?`) null "ClampVelocity" (0.0 0.0 0.0) 800.0 true
    (:`then`
      (bind _returnvalue_3 (`|SpawnActorFromClass` "/Game/Blueprints/Hitboxes/Hitbox.Hitbox_C" (`KismetMathLibrary.MakeTransform` (.location (`.Root` (`self.GetSockets`))) (struct) (5.0 5.0 5.0)) "Undefined" "MultiplyWithRoot" null 0.0 false false self true 1500.0 0.005 false null))
      (bind _output_get (set `self.HitBox` _returnvalue_3))
      (`Actor.K2_AttachToActor` _output_get _returnvalue_2 "None" "KeepWorld" "KeepWorld" "KeepWorld" true)
      (`GameplayStatics.PlaySoundAtLocation` "/Game/Audio/Player/Sword/ShimmerDash.ShimmerDash" (`Actor.K2_GetActorLocation` _returnvalue_2) (struct) 1.0 1.0 0.0 null null null null))
    (:`OnFinish`
      (`KismetSystemLibrary.Delay` 0.2)
      (`self.K2_EndAbility`))))

(event `self.K2_OnEndAbility`
  (params (bWasCancelled :type Boolean))
  (`parent.K2_OnEndAbility` bWasCancelled)
  (`|ExecutionSequence`
    (:`then_0`
      (`self.SetSelfCollision` "ECR_Block")
      (`Actor.K2_DestroyActor` (`self.HitBox`)))
    (:`then_1`
      ; Resume Movement
      (`Controller.ResetIgnoreMoveInput` (`.PlayerController` (break `GameplayAbilityActorInfo` (`self.GetActorInfo`)))))))
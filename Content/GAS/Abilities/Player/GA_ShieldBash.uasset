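; Player Shield Bash gameplay ability, activated from an event, that plays a montage and spawns a brief hitbox during it.
; An anim notify gameplay event spawns an enlarged hitbox just below the right hand socket, passing the ability as its reference.
; The hitbox expires after a fraction of a second, and the ability ends when the montage completes, blends out, is interrupted or is cancelled.
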(event `self.K2_ActivateAbilityFromEvent`
  (params (EventData :type "GameplayEventData Structure (by ref)"))
  (`parent.K2_ActivateAbilityFromEvent` EventData)
  (`GSCTask_PlayMontageWaitForEvent.PlayMontageAndWaitForEvent` "None" (`self.Montage to Play`) (struct :`GameplayTags` (struct :`(TagName` "Event.Anim.Notify")))
    (:`OnCompleted`
      (`self.K2_EndAbility` :!label _label))
    (:`OnBlendOut`
      (goto _label))
    (:`OnInterrupted`
      (goto _label))
    (:`OnCancelled`
      (goto _label))
    (:`EventReceived`
      (bind _returnvalue (`|SpawnActorFromClass` "/Game/Blueprints/Hitboxes/Hitbox.Hitbox_C" (`KismetMathLibrary.MakeTransform` (+ (.location (`.RightHand` (`self.GetSockets`))) (0.0 0.0 -50.0)) (struct) (4.0 4.0 4.0)) "Undefined" "MultiplyWithRoot" null 5.0 false false self true 500.0 null))
      (`Actor.SetLifeSpan` _returnvalue 0.1))))

(event `self.K2_OnEndAbility`
  (params (bWasCancelled :type Boolean))
  (`parent.K2_OnEndAbility` bWasCancelled))
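; Player gameplay ability that chooses between the two shield attacks, slam and bash, based on whether the character is airborne.
; On activation it checks if the avatar's character movement is falling, sends the Attack.Shield.Slam event if so or Attack.Shield.Bash otherwise, then ends immediately.
; It acts only as a dispatcher, leaving the attack itself to whatever responds to those gameplay event tags.
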(event `self.K2_ActivateAbility`
  (`parent.K2_ActivateAbility`)
  (`self.SendGameplayEvent` (select `bool` (`NavMovementComponent.IsFalling` (`Character.CharacterMovement` (cast `Character` (`self.GetAvatarActorFromActorInfo`) :!pure true))) :`false` (struct :`TagName` "Attack.Shield.Bash") :`true` (struct :`TagName` "Attack.Shield.Slam") :!type "GameplayTag Structure") (make `GameplayEventData` (struct)))
  (`self.K2_EndAbility`))

(event `self.K2_OnEndAbility`
  (params (bWasCancelled :type Boolean))
  (`parent.K2_OnEndAbility` bWasCancelled))
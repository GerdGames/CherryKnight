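; Base gameplay ability for character hit reactions, triggered by a gameplay event.
; It plays an optional montage and ends when that finishes or is interrupted, or after a brief delay if none is set.
; Unless the owner has the player blocking tag, it shows a red flash with hurt and hit sounds; otherwise it plays only a block sound.
; Ending the ability clears the red flash.
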(event `self.K2_ActivateAbilityFromEvent`
  (params (EventData :type "GameplayEventData Structure (by ref)"))
  (bind _owneractor (break `GameplayAbilityActorInfo` (`self.GetActorInfo`)))
  (bind _montage_to_play (`self.Montage to Play`)
    (:`then`
      (`AbilityTask_PlayMontageAndWait.CreatePlayMontageAndWaitProxy` "None" _montage_to_play 1.0 "None" false
        (:`then`
          (if (not (`GameplayTagAssetInterface.HasMatchingGameplayTag` (`.AbilitySystemComponent` (break `GameplayAbilityActorInfo` (`self.GetActorInfo`))) (struct :`TagName` "Character.Player.Blocking"))) :!label _label
            ; Hurt FX
            (`self.RedFlash` true)
            (bind _asbp_character_base (cast `/Game/Characters/BP_CharacterBase` _owneractor))
            (`GameplayStatics.PlaySoundAtLocation` (`/Game/Characters/BP_CharacterBase.HurtSoundCue` _asbp_character_base) (`Actor.K2_GetActorLocation` _owneractor) (struct) 1.0 1.0 0.0 null null null null)
            (`GameplayStatics.PlaySoundAtLocation` "/Game/Audio/Enemies/Hit/Light_Hit_Cue.Light_Hit_Cue" (`Actor.K2_GetActorLocation` _owneractor) (struct) 1.0 1.0 0.0 null null null null)
            (else
              ; Blocked hit
              (`GameplayStatics.PlaySoundAtLocation` "/Game/Audio/Player/Sword/Block_Cue.Block_Cue" (`Actor.K2_GetActorLocation` (`.OwnerActor` (break `GameplayAbilityActorInfo` (`self.GetActorInfo`)))) (struct) 1.0 1.0 0.0 null null null null))))
        (:`OnCompleted`
          (`self.K2_EndAbility` :!label _label_2))
        (:`OnBlendOut`
          (goto _label_2))
        (:`OnInterrupted`
          (goto _label_2))
        (:`OnCancelled`
          (goto _label_2))))
    (:`else`
      (`|ExecutionSequence`
        (:`then_0`
          (goto _label))
        (:`then_1`
          (`GameplayTask_WaitDelay.TaskWaitDelay` null 0.2
            (:`OnFinish`
              (goto _label_2))))))))

(event `self.K2_OnEndAbility`
  (params (bWasCancelled :type Boolean))
  (`parent.K2_OnEndAbility` bWasCancelled)
  (`self.RedFlash` false))
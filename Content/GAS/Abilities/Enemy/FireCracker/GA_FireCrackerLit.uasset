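; Gameplay ability for the FireCracker enemy that emits repeated small blasts at the avatar's location once lit.
; Event activation starts an endless loop that spawns a Hitbox scaled by ExplosionSize, flagged as fuse-lighting blast damage without knockback.
; Each hitbox is destroyed next tick, then the loop waits Period plus slight random jitter and prints a debug "crac" per pop.
; The graph never calls EndAbility itself.
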(event `self.K2_ActivateAbilityFromEvent`
  (params (EventData :type "GameplayEventData Structure (by ref)"))
  (`KismetSystemLibrary.PrintString` "crac" :!label _label)
  (bind _returnvalue (`|SpawnActorFromClass` "/Game/Blueprints/Hitboxes/Hitbox.Hitbox_C" (`KismetMathLibrary.MakeTransform` (`Actor.K2_GetActorLocation` (`self.GetAvatarActorFromActorInfo`)) (struct) (`KismetMathLibrary.Conv_DoubleToVector` (`self.ExplosionSize`))) "Undefined" "MultiplyWithRoot" null 5.0 true true self false 500.0 null))
  (`KismetSystemLibrary.DelayUntilNextTick`)
  (`Actor.K2_DestroyActor` _returnvalue)
  (`KismetSystemLibrary.Delay` (+ (`self.Period`) (`KismetMathLibrary.RandomFloatInRange` 0.0 0.1)))
  (goto _label))
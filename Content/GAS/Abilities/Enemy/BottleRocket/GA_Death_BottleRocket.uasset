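; Death ability for the Bottle Rocket enemy, which launches it upward and homes it into a nearby pillar.
; It red-flashes, plays an optional montage and rises via a root motion MoveTo force.
; A sphere overlap picks the nearest BP_Pillar not tagged dead, and a MoveToActor force flies the enemy at it.
; FinalizeDeath follows a short delay after arrival; finding no pillar just ends the ability.
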(event `self.K2_ActivateAbilityFromEvent`
  (params (EventData :type "GameplayEventData Structure (by ref)"))
  (bind _homingactor (`self.HomingActor`))
  (bind _actors_to_ignore (`self.Actors to Ignore`))
  (`self.RedFlash` true)
  (`KismetArrayLibrary.Array_Add` _actors_to_ignore (`GameplayStatics.GetPlayerCharacter` 0))
  (`KismetArrayLibrary.Array_Add` _actors_to_ignore (`self.GetAvatarActorFromActorInfo`))
  (if (`KismetArrayLibrary.Array_IsNotEmpty` (`self.Montage to Play`))
    (`AbilityTask_PlayMontageAndWait.CreatePlayMontageAndWaitProxy` "None" null 1.0 "None" false
      (:`then`
        _)))
  (`AbilityTask_ApplyRootMotionMoveToForce.ApplyRootMotionMoveToForce` "None" (+ (`Actor.K2_GetActorLocation` (`self.GetAvatarActorFromActorInfo`)) (0.0 0.0 800.0)) 1.0 false "MOVE_None" false null "MaintainLastRootMotionVelocity"
    (:`OnTimedOut`
      _)
    (:`OnTimedOutAndDestinationReached`
      _))
  (bind (_returnvalue _outactors) (`self.FindHoming` "/Game/Blueprints/Pillars/BP_Pillar.BP_Pillar_C" :!label _label))
  (if _returnvalue
    (set `self.HomingActor` (`.ReturnValue` (`GameplayStatics.FindNearestActor` (`Actor.K2_GetActorLocation` (`self.GetAvatarActorFromActorInfo`)) _outactors)))
    (if (not (`GSCBlueprintFunctionLibrary.HasMatchingGameplayTag` _homingactor (struct :`TagName` "Character.Hit.Dead"))) :!label _label_2
      (`AbilityTask_ApplyRootMotionMoveToActorForce.ApplyRootMotionMoveToActorForce` "None" _homingactor (0.0 0.0 0.0) "AlignFromTargetToSource" 1.0 null null false "MOVE_None" false null null "MaintainLastRootMotionVelocity" (0.0 0.0 0.0) 0.0 false 300.0
        (:`then`
          (`Actor.K2_SetActorRotation` (`self.GetAvatarActorFromActorInfo`) (struct :`Yaw` 90.0) false))
        (:`OnFinished`
          (`KismetSystemLibrary.Delay` 1.0)
          (`self.FinalizeDeath`)))
      (else
        (`KismetArrayLibrary.Array_Add` (`self.Actors to Ignore`) _homingactor)
        (goto _label)))
    (else
      (bind (_returnvalue_2 _outactors_2) (`self.FindHoming` "/Game/Blueprints/Pillars/BP_Pillar.BP_Pillar_C"))
      (if _returnvalue_2
        (set `self.HomingActor` (`KismetArrayLibrary.Array_Random` _outactors_2))
        (goto _label_2)
        (else
          (`self.K2_EndAbility`))))))

(fn `FindHoming`
  (params (ActorClassFilter :type "Object Class Reference"))
  (returns (ReturnValue :type Boolean) (OutActors :type "Array of Actor Object Reference"))
  (bind (_outactors _returnvalue) (`KismetSystemLibrary.SphereOverlapActors` (`Actor.K2_GetActorLocation` (`self.GetAvatarActorFromActorInfo`)) (`self.Sphere Radius`) (`|MakeArray` "ObjectTypeQuery3" :!type "EObjectTypeQuery Enum") ActorClassFilter (`self.Actors to Ignore`)))
  (return _returnvalue _outactors))
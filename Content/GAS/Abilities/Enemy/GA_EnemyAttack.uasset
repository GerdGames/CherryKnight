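; Gameplay ability for an enemy melee attack that damages and optionally knocks back the player.
; It plays an optional montage and strikes on an anim notify event, ending when the montage completes.
; A strike sphere-overlaps for the Cherry Knight player in front of the avatar, draws a debug sphere and calls DealDamage on hits.
; Without a montage, it strikes once after a short delay, then ends.
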(event `self.K2_ActivateAbility`
  (bind _returnvalue (`self.GetAvatarActorFromActorInfo`))
  (bind _attackradius (`self.AttackRadius`))
  (bind _returnvalue_2 (+ (`Actor.K2_GetActorLocation` _returnvalue) (* (`Actor.GetActorForwardVector` _returnvalue) (`self.ForwardOffset`))))
  (`parent.K2_ActivateAbility`)
  (bind _montage_to_play (`self.Montage to Play`)
    (:`then`
      (`GSCTask_PlayMontageWaitForEvent.PlayMontageAndWaitForEvent` "None" _montage_to_play (struct :`GameplayTags` (struct :`(TagName` "Event.Anim.Notify")))
        (:`OnCompleted`
          (`self.K2_EndAbility`))
        (:`EventReceived`
          (`KismetSystemLibrary.DrawDebugSphere` _returnvalue_2 _attackradius 12 (struct :`R` 1.0 :`B` 0.004858 :`A` 1.0) 0.1 3.0 :!label _label)
          (bind _outactors (`KismetSystemLibrary.SphereOverlapActors` _returnvalue_2 _attackradius (`|MakeArray` "ObjectTypeQuery3" :!type "EObjectTypeQuery Enum") "/Game/Characters/BP_CherryKnightPlayer.BP_CherryKnightPlayer_C"))
          (for _array_element _outactors
            (`self.DealDamage` _array_element (`self.Damage`) false false (`self.Knock Back?`) (`self.Knock Magnitude`))))))
    (:`else`
      (`KismetSystemLibrary.Delay` 0.5)
      (`|ExecutionSequence`
        (:`then_0`
          (goto _label))
        (:`then_1`
          (`self.K2_EndAbility`))))))
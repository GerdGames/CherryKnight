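; Gameplay ability that moves the small bomb enemy toward its AI destination with a single hop.
; On activation it reads the Destination vector from the avatar's Blackboard and launches a root motion jump force facing that point.
; Jump distance is the horizontal gap capped at a short maximum, and height is the absolute vertical gap plus padding.
; The ability ends when the Landed callback fires.
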(event `self.K2_ActivateAbility`
  (bind _returnvalue (`self.GetAvatarActorFromActorInfo`))
  (bind _returnvalue_2 (`Actor.K2_GetActorLocation` _returnvalue))
  (bind _returnvalue_3 (`BlackboardComponent.GetValueAsVector` (`AIBlueprintHelperLibrary.GetBlackboard` _returnvalue) "Destination"))
  (`parent.K2_ActivateAbility`)
  (`AbilityTask_ApplyRootMotionJumpForce.ApplyRootMotionJumpForce` "None" (`KismetMathLibrary.FindLookAtRotation` _returnvalue_2 _returnvalue_3) (`KismetMathLibrary.FClamp` (`KismetMathLibrary.Vector_Distance` (`KismetMathLibrary.MakeVector` (.x _returnvalue_2) (.y _returnvalue_2)) (`KismetMathLibrary.MakeVector` (.x _returnvalue_3) (.y _returnvalue_3))) 0.0 150.0) (+ (`KismetMathLibrary.Vector_Distance` (`KismetMathLibrary.MakeVector` 0.0 0.0 (.z _returnvalue_2)) (`KismetMathLibrary.MakeVector` 0.0 0.0 (.z _returnvalue_3))) 50.0) 0.5 1.0 true "MaintainLastRootMotionVelocity"
    (:`OnLanded`
      (`self.K2_EndAbility`))))
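; Base death Gameplay Ability that flashes the avatar red, plays a random death montage, then removes the actor.
; An anim notify event finalizes death immediately, while montage end, interruption or an empty montage list finalizes it after DeathDelay.
; Finalizing optionally explodes, dealing blast damage with configurable knockback and fuse lighting to overlapped pawns and drawing a debug sphere.
; It then sets a tiny randomized lifespan to destroy the avatar.
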(event `self.K2_ActivateAbilityFromEvent`
  (params (EventData :type "GameplayEventData Structure (by ref)"))
  (bind _montage_to_play (`self.Montage to Play`))
  (`self.RedFlash` true)
  (if (`KismetArrayLibrary.Array_IsNotEmpty` _montage_to_play)
    (`GSCTask_PlayMontageWaitForEvent.PlayMontageAndWaitForEvent` "None" (`KismetArrayLibrary.Array_Random` _montage_to_play) (struct :`GameplayTags` (struct :`(TagName` "Event.Anim.Notify")))
      (:`OnCompleted`
        (`KismetSystemLibrary.Delay` (`self.DeathDelay`) :!label _label))
      (:`OnBlendOut`
        (goto _label))
      (:`OnInterrupted`
        (goto _label))
      (:`OnCancelled`
        (goto _label))
      (:`EventReceived`
        _))
    (else
      (goto _label)))
  (`self.FinalizeDeath`))

(event `self.K2_OnEndAbility`
  (params (bWasCancelled :type Boolean))
  (`parent.K2_OnEndAbility` bWasCancelled))

(fn `DeathLifeSpan`
  (`Actor.SetLifeSpan` (`self.GetAvatarActorFromActorInfo`) (`KismetMathLibrary.RandomFloatInRange` 0.01 0.1)))

(fn `Explode`
  (bind _exploderadius (`self.ExplodeRadius`))
  (bind _returnvalue (`Actor.K2_GetActorLocation` (`self.GetAvatarActorFromActorInfo`)))
  (if (`self.Explodes?`)
    (`KismetSystemLibrary.DrawDebugSphere` _returnvalue _exploderadius 12 (struct :`R` 1.0 :`G` 0.108501 :`A` 1.0) 0.2 2.0)
    (bind _outactors (`KismetSystemLibrary.SphereOverlapActors` _returnvalue _exploderadius (`|MakeArray` "ObjectTypeQuery3" :!type "EObjectTypeQuery Enum")))
    (for _array_element _outactors
      (`self.DealDamage` _array_element (`self.ExplodeDamage`) (`self.ExplosionLightsFuse?`) true (`self.ExplosionKnocks?`) (`self.KnockMagnitude`)))))

(fn `FinalizeDeath`
  (`self.Explode`)
  (`self.DeathLifeSpan`))
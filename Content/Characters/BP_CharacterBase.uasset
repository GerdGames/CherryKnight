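; Base character Blueprint that handles death through the Gameplay Ability System.
; On BeginPlay it keeps a repeating attribute-change listener, apparently on health judging by leftover debug text.
; When the changed value falls to zero or below, it sends itself a Character.Hit.Dead gameplay event, leaving the response to whatever handles that tag.
; The death sound plays at the actor's location on Destroyed, separately from that event.
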(event `self.ReceiveBeginPlay`
  (`parent.ReceiveBeginPlay`)
  (bind (_asynctaskproxy _attribute _newvalue _oldvalue) (`AbilityAsync_WaitAttributeChanged.WaitForAttributeChanged` null (struct :`AttributeName` "CurrentHealth" :`Attribute` "/Game/GAS/Attributes/GBA_AttributesBase.GBA_AttributesBase_C:CurrentHealth" :`AttributeOwner` "/Script/Engine.BlueprintGeneratedClass'/Game/GAS/Attributes/GBA_AttributesBase.GBA_AttributesBase_C'"))
    (:`Changed`
      (if (!= _newvalue _oldvalue)
        (if (<= _newvalue 0.0)
          (`AbilitySystemBlueprintLibrary.SendGameplayEventToActor` self (struct :`TagName` "Character.Hit.Dead")))))))

(event `self.ReceiveDestroyed`
  (`GameplayStatics.PlaySoundAtLocation` (`self.DeathSoundCue`) (`self.K2_GetActorLocation`) (struct) 1.0 1.0 0.0 null null null null))

(fn `UserConstructionScript`)
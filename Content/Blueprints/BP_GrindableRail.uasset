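; Spline-built grind rail that latches a player and carries them along it until ejection.
; The construction script tiles instanced meshes along the spline and caches their world transforms as rail points.
; InitiateGrind lerps the player to the rail, sends a Latched gameplay event, then picks the nearest point and a direction from the player's forward vector.
; A replayed timeline steps GrindPositionPoint between points, Tick pins the player above it, and ejection launches the character off.
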(event `self.ReceiveBeginPlay`
  ; Comment
  (`TimelineComponent.SetPlayRate` (`self.InterpBetweenPoints`) 15.0)
  (`TimelineComponent.SetPlayRate` (`self.InterpToRail`) 5.0))

(event `self.ReceiveTick`
  (params (DeltaSeconds :type "Float (single-precision)"))
  (bind (_returnvalue_x _returnvalue_y _returnvalue_z) (`KismetMathLibrary.BreakVector` (`SceneComponent.K2_GetComponentLocation` (`self.GrindPositionPoint`))))
  ; TICK
  (bind _player (`self.Player`)
    (:`then`
      (`self.K2_SetActorLocation` _player (`KismetMathLibrary.MakeVector` _returnvalue_x _returnvalue_y (+ _returnvalue_z 70.0)) false false))
    (:`else`)))

(event `/Game/Blueprints/BPI_Grinding.InitiateGrind`
  (params (ForwardVector :type "Vector Structure") (InitalPlayerLocation :type "Vector Structure") (Player :type "Actor Object Reference"))
  (bind _startindex (`self.StartIndex`))
  (bind (_playergrindpoint_x _playergrindpoint_y _playergrindpoint_z) (`KismetMathLibrary.BreakVector` (`self.PlayerGrindPoint`)))
  ; start
  (set `self.Player Forward Vector` ForwardVector)
  (set `self.PlayerGrindPoint` InitalPlayerLocation)
  (set `self.Player` Player)
  (bind _output_get (set `self.InitialInterpStart` (`self.K2_GetActorLocation` (`self.Player`))))
  (bind (_direction _alpha) (`Timeline|InterpToRail` :!via `PlayFromStart`)
    (:`Update`
      (bind _player (`self.Player`)
        (:`then`
          (`self.K2_SetActorLocation` _player (`KismetMathLibrary.VLerp` _output_get (`KismetMathLibrary.MakeVector` _playergrindpoint_x _playergrindpoint_y (+ _playergrindpoint_z 70.0)) _alpha) false false))
        (:`else`)))
    (:`Finished`
      (bind _player_2 (`self.Player`)
        (:`then`
          (`AbilitySystemBlueprintLibrary.SendGameplayEventToActor` _player_2 (struct :`TagName` "Movement.Grinding.Latched") (make `GameplayEventData` (struct))))
        (:`else`
          _))
      (bind _outnearestindex (`self.FindNearestRailPointIndex` (`self.PlayerGrindPoint`)))
      (bind (_output_location _output_rotation) (`KismetMathLibrary.BreakTransform` (`|GetArrayItem` (`self.RailSpawnTransforms`) _outnearestindex)))
      (`self.RoundGrindDirection` _output_rotation)
      (set `self.StartIndex` _outnearestindex)
      (`KismetSystemLibrary.DrawDebugPoint` _output_location 50.0 (struct :`G` 0.098949 :`B` 1.0 :`A` 1.0) 5.0)
      (set `self.LastGrindIndex` _startindex)
      (set `self.CurrentGrindIndex` _startindex)
      (`self.StartGrinding`))))

(event `StageGrind`
  (bind _currentgrindindex (`self.CurrentGrindIndex`))
  (bind _output_location (`KismetMathLibrary.BreakTransform` (`|GetArrayItem` (`self.RailSpawnTransforms`) (`self.CurrentGrindIndex`))))
  (bind _output_location_2 (`KismetMathLibrary.BreakTransform` (`|GetArrayItem` (`self.RailSpawnTransforms`) (+ (`self.CurrentGrindIndex`) (`self.Direction`)))))
  ; StartGrinding
  (bind (_direction _alpha) (`Timeline|InterpBetweenPoints` :!via `PlayFromStart` :!label _label)
    (:`Update`
      (if (== (`KismetMathLibrary.VSize` _output_location_2) 0.0)
        (message `/Game/Blueprints/BPI_Grinding.Eject` (`self.Player`))
        (else
          (`SceneComponent.K2_SetWorldLocation` (`self.GrindPositionPoint`) (`KismetMathLibrary.VLerp` _output_location _output_location_2 _alpha) false false))))
    (:`Finished`
      (set `self.CurrentGrindIndex` (+ (`self.CurrentGrindIndex`) (`self.Direction`)))
      (if (or (< _currentgrindindex 0) (> _currentgrindindex (- (`KismetArrayLibrary.Array_Length` (`self.RailSpawnTransforms`)) 1)))
        (`self.EjectPlayer`)
        (elif (`self.StageGrindBool`)
          (`self.StageGrind`)
          (`KismetSystemLibrary.PrintString` (`KismetStringLibrary.Conv_IntToString` (`self.CurrentGrindIndex`))))))))

(event `StopInterpTimeline`
  ; StartGrinding
  (goto _label :!via `Stop`))

(event `StartGrinding`
  (bind _output_location (`KismetMathLibrary.BreakTransform` (`|GetArrayItem` (`self.RailSpawnTransforms`) (`self.CurrentGrindIndex`))))
  ; StartGrinding
  (`SceneComponent.K2_SetWorldLocation` (`self.GrindPositionPoint`) _output_location false false)
  (set `self.StageGrindBool` true)
  (goto _label :!via `PlayFromStart`))

(event `EjectPlayer`
  (bind _player (`self.Player`))
  (bind _lauchscale (`self.LauchScale`))
  ; stop
  (message `/Game/Blueprints/BPI_Grinding.EjectPlayerMessage` _player)
  (bind _ascharacter (cast `Character` _player))
  (set `self.StageGrindBool` false)
  (bind (_returnvalue_x _returnvalue_y) (`KismetMathLibrary.BreakVector` (`self.GetActorForwardVector` _ascharacter)))
  (`Character.LaunchCharacter` _ascharacter (`KismetMathLibrary.MakeVector` (* _returnvalue_x _lauchscale) (* _returnvalue_y _lauchscale) 1000.0) false false)
  (set `self.Player` null)
  (`KismetSystemLibrary.PrintString` "PLAYER EJECTED")
  (`self.StopInterpTimeline`)
  ;; Comment
  (`self.resetGrindPos`))

(event `resetGrindPos`
  ; stop
  ;; Comment
  (`SceneComponent.K2_SetRelativeLocation` (`self.GrindPositionPoint`) (0.0 0.0 0.0) false false)
  (set `self.CurrentGrindIndex` 0)
  (set `self.StartIndex` 0))

(event `/Game/Blueprints/BPI_Grinding.EjectRailMessage`
  ; stop
  (`self.EjectPlayer`))

(fn `FindNearestRailPointIndex`
  (params (InitialPlayerLocation :type "Vector Structure"))
  (returns (OutNearestIndex :type Integer))
  (locals (Distance :type "Float (double-precision)" :default 999.0) (NearestIndex :type Integer))
  (for (_array_element _array_index) (`self.RailSpawnTransforms`)
    (bind _returnvalue (`KismetMathLibrary.Vector_Distance` (.location _array_element) InitialPlayerLocation))
    (if (< _returnvalue (`local.Distance`))
      (set `local.Distance` _returnvalue)
      (set `local.NearestIndex` _array_index)))
  (return (`local.NearestIndex`)))

(fn `GetPlayerTargetedRailingData`
  (returns (Actor :type "Actor Object Reference") (Location :type "Vector Structure"))
  (return null (0.0 0.0 0.0)))

(fn `RoundGrindDirection`
  (params (InRot :type "Rotator Structure"))
  (bind _returnvalue (`KismetMathLibrary.Dot_VectorVector` (`KismetMathLibrary.Conv_RotatorToVector` InRot) (`self.Player Forward Vector`)))
  (if (> _returnvalue 0.0)
    (set `self.Direction` (`KismetMathLibrary.FCeil` _returnvalue))
    (else
      (set `self.Direction` (`KismetMathLibrary.FFloor` _returnvalue))))
  (return))

(fn `UpdateGrindLocationOnSpline`
  (params (`Player Location` :type "Vector Structure"))
  (returns (UpdatedGrindLocation :type "Vector Structure"))
  (return (0.0 0.0 0.0)))

(fn `UserConstructionScript`
  (locals (Instances :type Integer :default 0))
  (bind _mesh (`self.Mesh`))
  (bind _spline (`self.Spline`))
  (bind (_returnvalue_min _returnvalue_max) (break `Box` (`StaticMesh.GetBoundingBox` _mesh)))
  (bind _returnvalue_x (`KismetMathLibrary.BreakVector` (- _returnvalue_max _returnvalue_min)))
  (`StaticMeshComponent.SetStaticMesh` (`self.InstancedStaticMesh`) _mesh)
  (bind _output_get (set `local.Instances` (`KismetMathLibrary.FFloor` (/ (`SplineComponent.GetSplineLength` (`self.Spline`)) _returnvalue_x))))
  (for _index (range (+ _output_get 1))
    (bind _returnvalue (`SplineComponent.GetLocationAtDistanceAlongSpline` _spline (* _index _returnvalue_x) "Local"))
    (bind _returnvalue_2 (`InstancedStaticMeshComponent.AddInstance` (`self.InstancedStaticMesh`) (`KismetMathLibrary.MakeTransform` _returnvalue (`KismetMathLibrary.FindLookAtRotation` _returnvalue (`SplineComponent.GetLocationAtDistanceAlongSpline` _spline (* (+ _index 1) _returnvalue_x) "Local"))) false))
    (bind _outinstancetransform (`InstancedStaticMeshComponent.GetInstanceTransform` (`self.InstancedStaticMesh`) _returnvalue_2 true))
    (`KismetArrayLibrary.Array_AddUnique` (`self.RailSpawnTransforms`) (`KismetMathLibrary.MakeTransform` (`KismetMathLibrary.MakeVector` (.x (.location _outinstancetransform)) (.y (.location _outinstancetransform)) (.z (.location _outinstancetransform))) (.rotation _outinstancetransform) (.scale _outinstancetransform)))))
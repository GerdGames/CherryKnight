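; BP_Pillar is a destructible pillar whose destruction is reported to a manager for the win condition.
; BeginPlay watches a GAS Companion attribute, mapping its ratio to five damage states that drive mesh swaps, a crumble sound and hiding the flame.
; Both the zero-value check and UpdateDamageVisuals can call CallPillarDestroyed, through separate DoOnce gates.
; Separate CurrentHealth-based damage functions exist but are not called in this graph.
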(event `self.ReceiveBeginPlay`
  (bind (_asynctaskproxy _attribute _newvalue) (`AbilityAsync_WaitAttributeChanged.WaitForAttributeChanged` null (struct :`AttributeName` "CurrentHealth" :`Attribute` "/Game/GAS/Attributes/GBA_AttributesBase.GBA_AttributesBase_C:CurrentHealth" :`AttributeOwner` "/Script/Engine.BlueprintGeneratedClass'/Game/GAS/Attributes/GBA_AttributesBase.GBA_AttributesBase_C'"))
    (:`Changed`
      (`|ExecutionSequence`
        (:`then_0`
          (bind _returnvalue (`KismetMathLibrary.Abs_Int` (`KismetMathLibrary.FCeil` (* (/ _newvalue (`.ReturnValue` (`AbilitySystemComponent.GetGameplayAttributeValue` (`self.GSCAbilitySystem`) (struct :`AttributeName` "MaxHealth" :`Attribute` "/Game/GAS/Attributes/GBA_AttributesBase.GBA_AttributesBase_C:MaxHealth" :`AttributeOwner` "/Script/Engine.BlueprintGeneratedClass'/Game/GAS/Attributes/GBA_AttributesBase.GBA_AttributesBase_C'")))) -5.0))))
          (bind _returnvalue_2 (select `int` _returnvalue :`0` "NewEnumerator4" :`1` "NewEnumerator3" :`2` "NewEnumerator2" :`3` "NewEnumerator1" :`4` "NewEnumerator0" :!type "/Game/Blueprints/Pillars/E_Pillar_DamageStates Enum"))
          ; Check if the new pillar state is different from the old one To update damage videos and play sound effect
          (if (`|EnumInequality` _returnvalue_2 (`self.DamageState`))
            (`KismetSystemLibrary.PrintString` (`KismetStringLibrary.Conv_IntToString` _returnvalue))
            (set `self.DamageState` _returnvalue_2)
            (`self.UpdateDamageVisuals`)
            (`GameplayStatics.PlaySoundAtLocation` "/Game/Audio/Pillar/PillarCrumble_Cue.PillarCrumble_Cue" (`self.K2_GetActorLocation`) (struct) 1.0 1.0 0.0 null null null null)))
        (:`then_1`
          ; Destroy pillar if at 0 or below
          ;;[1 0 0 0.5] This needs to be called when pillar is destroyed to let the manager know. Win condition is dependent on it
          (if (<= _newvalue 0.0)
            (`/Engine/EditorBlueprintResources/StandardMacros.DoOnce` false
              (:`Completed`
                (`self.PillarDestroyed`)))))))))

(fn `SetDamageState`
  (locals (DamageQuarterAmount :type "Float (double-precision)"))
  (set `local.DamageQuarterAmount` (/ (`self.MaxHealth`) 4.0))
  (if (>= (`self.CurrentHealth`) (`self.MaxHealth`))
    (set `self.DamageState` "NewEnumerator0")
    (elif (>= (`self.CurrentHealth`) (* (`local.DamageQuarterAmount`) 3.0))
      (set `self.DamageState` "NewEnumerator1")
      (elif (>= (`self.CurrentHealth`) (* (`local.DamageQuarterAmount`) 2.0))
        (set `self.DamageState` "NewEnumerator2")
        (elif (>= (`self.CurrentHealth`) (* (`local.DamageQuarterAmount`) 1.0))
          (set `self.DamageState` "NewEnumerator3")
          (else
            (if (<= (`self.CurrentHealth`) 0.0)
              _
              (else
                _))
            (set `self.DamageState` "NewEnumerator4"))))))
  (return))

(fn `SetupDefaults`
  ; Set starting health
  (set `self.CurrentHealth` (`self.MaxHealth`))
  (`self.UpdateDamageVisuals`)
  (return))

(fn `TakeDamage`
  (params (IncomingDamage :type "Float (double-precision)"))
  (set `self.CurrentHealth` (`KismetMathLibrary.FClamp` (- (`self.CurrentHealth`) IncomingDamage) 0.0 (`self.MaxHealth`)))
  (return))

(fn `UpdateDamageVisuals`
  (bind _damagestate (`self.DamageState`))
  (bind _returnvalue (select `/Game/Blueprints/Pillars/E_Pillar_DamageStates` _damagestate :`NewEnumerator4` true))
  (`StaticMeshComponent.SetStaticMesh` (`self.Pillar_Mesh`) (select `/Game/Blueprints/Pillars/E_Pillar_DamageStates` _damagestate :`NewEnumerator0` "/Game/Art/Mesh/EnvironmentKit/Pillar_A.Pillar_A" :`NewEnumerator1` "/Game/Art/Mesh/EnvironmentKit/Pillar_A1.Pillar_A1" :`NewEnumerator2` "/Game/Art/Mesh/EnvironmentKit/Pillar_A2.Pillar_A2" :`NewEnumerator3` "/Game/Art/Mesh/EnvironmentKit/Pillar_A3.Pillar_A3" :`NewEnumerator4` "/Game/Art/Mesh/EnvironmentKit/Pillar_B.Pillar_B" :!type "StaticMesh Object Reference"))
  (`SceneComponent.SetHiddenInGame` (`self.Flame`) _returnvalue false)
  (`|ExecutionSequence`
    (:`then_0`
      (if _returnvalue
        (`/Engine/EditorBlueprintResources/StandardMacros.DoOnce` false
          (:`Completed`
            (`self.PillarDestroyed`)))))
    (:`then_1`
      (return))))

(fn `UserConstructionScript`)
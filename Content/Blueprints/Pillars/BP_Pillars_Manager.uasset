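; Manager that tracks how many BP_Pillar actors on the map have been destroyed.
; On BeginPlay it caches all pillars, binds to their destroyed events and warns if none exist.
; Each status check recounts pillars by DamageState, broadcasts destroyed and total counts through UpdatePillarCount, and prints a message when all are destroyed.
; CheckRemainingPillars also holds an unconnected early-exit version of the all-destroyed check.
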(event `self.ReceiveBeginPlay`
  (`self.StorePillarRefs`) ; Finds all pillars on map
  (bind _pillarsonmap (`self.VerifyPillarCount`)) ; Lets dev know how many pillars were found
  (`self.UpdatePillarCount` 0 _pillarsonmap))

(event `CheckPillarsStatus`
  (bind (_allpillarsdestroyed _destroyedpillars _totalpillars) (`self.CheckRemainingPillars`)) ; Checks to see if all pillars have been destroyed
  (`self.UpdatePillarCount` _destroyedpillars _totalpillars)
  (if _allpillarsdestroyed
    (`KismetSystemLibrary.PrintString` "ALL PILLARS DESTROYED")))

(fn `CheckRemainingPillars`
  (returns (AllPillarsDestroyed :type Boolean) (DestroyedPillars :type Integer) (TotalPillars :type Integer))
  (locals (AtLeastOnePillarRemains :type Boolean) (TotalDestroyedPillars :type Integer))
  (bind _totaldestroyedpillars (`local.TotalDestroyedPillars`))
  (bind _returnvalue (`KismetArrayLibrary.Array_Length` (`self.AllPillars`)))
  (for _array_element (`self.AllPillars`)
    (if (`|EnumInequality` (`/Game/Blueprints/Pillars/BP_Pillar.DamageState` _array_element) "NewEnumerator4")
      (`/Engine/EditorBlueprintResources/StandardMacros.IncrementInt` (`local.TotalDestroyedPillars`))))
  (if (>= (`local.TotalDestroyedPillars`) (`KismetArrayLibrary.Array_Length` (`self.AllPillars`)))
    (return true _totaldestroyedpillars _returnvalue)
    (else
      (return false _totaldestroyedpillars _returnvalue))))

(fn `StorePillarRefs`
  (bind _outactors (`GameplayStatics.GetAllActorsOfClass` "/Game/Blueprints/Pillars/BP_Pillar.BP_Pillar_C"))
  (bind _output_get (set `self.AllPillars` _outactors))
  (for _array_element _output_get
    (add `/Game/Blueprints/Pillars/BP_Pillar.PillarDestroyed` _array_element (`|CreateDelegate` :!event `CheckPillarsStatus`)))
  (return))

(fn `UserConstructionScript`)

(fn `VerifyPillarCount`
  (returns (PillarsOnMap :type Integer))
  (if (`KismetArrayLibrary.Array_IsEmpty` (`self.AllPillars`))
    (`KismetSystemLibrary.PrintString` "WARNING: NO PILLARS ON MAP!" true true (struct :`R` 1.0 :`G` 0.038007 :`B` 0.003498 :`A` 1.0))
    (return 0)
    (else
      (return (`KismetArrayLibrary.Array_Length` (`self.AllPillars`))))))
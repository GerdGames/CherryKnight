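; Firecracker projectile that launches in a random, upward-biased direction and explodes after a short random lifespan.
; The construction script randomizes the projectile velocity, and Tick moves a lit-fuse Niagara effect along with the actor.
; On destruction, it spawns a brief, scaled-up Hitbox that inherits its damage, knockback and ability settings, then swaps the fuse effect for an explosion.
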(event `self.ReceiveBeginPlay`
  (`self.SetLifeSpan` (`KismetMathLibrary.RandomFloatInRange` 0.2 0.4))
  (bind _returnvalue (`NiagaraFunctionLibrary.SpawnSystemAtLocation` "/Game/Fireworks/CustomFx/LitSparks/ContinousLit_FX.ContinousLit_FX" (`self.K2_GetActorLocation`)))
  (set `self.SpawnedFX` _returnvalue))

(event `self.ReceiveDestroyed`
  (bind (_returnvalue_location _returnvalue_rotation) (`KismetMathLibrary.BreakTransform` (`self.GetTransform`)))
  (bind _returnvalue (`|SpawnActorFromClass` "/Game/Blueprints/Hitboxes/Hitbox.Hitbox_C" (`KismetMathLibrary.MakeTransform` _returnvalue_location _returnvalue_rotation (8.0 8.0 8.0)) "Undefined" "MultiplyWithRoot" null (`self.Damage`) (`self.Light Fuse?`) (`self.Is Blast Damage?`) (`self.AbilityReference`) (`self.Knock Back?`) (`self.Knock Magnitude`) null))
  (`self.SetLifeSpan` _returnvalue 0.1)
  (`ActorComponent.Deactivate` (`self.SpawnedFX`))
  (`NiagaraFunctionLibrary.SpawnSystemAtLocation` "/Game/Fireworks/CustomFx/Saturn_Explosion_FX.Saturn_Explosion_FX" (`self.K2_GetActorLocation`)))

(event `self.ReceiveTick`
  (params (DeltaSeconds :type "Float (single-precision)"))
  (`SceneComponent.K2_SetWorldLocation` (`self.SpawnedFX`) (`self.K2_GetActorLocation`) false false))

(fn `UserConstructionScript`
  (bind _returnvalue (`KismetMathLibrary.RandomFloat`))
  (bind _returnvalue_2 (`KismetMathLibrary.SelectFloat` _returnvalue (* _returnvalue -1.0) (`KismetMathLibrary.RandomBool`)))
  (set `MovementComponent.Velocity` (`KismetMathLibrary.MakeVector` _returnvalue_2 _returnvalue_2 (`KismetMathLibrary.RandomFloatInRange` 0.4 0.8)) (`self.ProjectileMovement`)))
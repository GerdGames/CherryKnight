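; Hitbox actor that deals damage on behalf of a gameplay ability to actors it overlaps.
; On overlap it skips the ability's avatar and anything already in EnemiesHit, so each actor is hit once per hitbox.
; It hands damage, knockback, blast and fuse settings to the ability's DealDamage, with hitstop switched off after the first target so only that hit can trigger it.
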(event `self.ReceiveActorBeginOverlap`
  (params (OtherActor :type "Actor Object Reference"))
  (bind _enemieshit (`self.EnemiesHit`))
  (`/Engine/EditorBlueprintResources/StandardMacros.IsValid` OtherActor
    (:`Is Valid`
      (if (!= OtherActor (`GameplayAbility.GetAvatarActorFromActorInfo` (`self.AbilityReference`)))
        (if (not (`KismetArrayLibrary.Array_Contains` _enemieshit OtherActor))
          (if (not (`KismetArrayLibrary.Array_IsEmpty` _enemieshit))
            (set `self.ApplyHitstop?` false))
          (`KismetArrayLibrary.Array_Add` _enemieshit OtherActor)
          (`/Game/GAS/Abilities/GA_AbilityBase.DealDamage` (`self.AbilityReference`) OtherActor (`self.Damage`) (`self.Light Fuse?`) (`self.Is Blast Damage?`) (`self.Knock Back?`) (`self.Knock Magnitude`) (`self.Hit Stop Duration`) (`self.ApplyHitstop?`)))))))

(fn `UserConstructionScript`)